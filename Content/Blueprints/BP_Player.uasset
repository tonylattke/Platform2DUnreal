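; Player character that switches between Box, Circle and Triangle forms, each with its own mesh, walk speed and skill.
; Enhanced Input drives sideways movement, pausing, skills and form switching, with GameMode choosing the next form and GameInstance holding the current one.
; Box shrinks while the skill is held and Tick regrows it after release.
; Circle dashes along world Y using the last move input, and Triangle jumps, both on skill completion.
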(event `self.ReceiveBeginPlay`
  (`self.SetupController`)
  (bind _asbp_game_mode (cast `/Game/Blueprints/BP_GameMode` (`GameplayStatics.GetGameMode`)))
  (set `self.MyGameMode` _asbp_game_mode)
  (bind _asbp_game_instance (cast `/Game/Blueprints/BP_GameInstance` (`GameplayStatics.GetGameInstance`)))
  (bind _output_get (set `self.MyGameInstance` _asbp_game_instance))
  (`self.UpdateMesh` (`/Game/Blueprints/BP_GameInstance.CurrentGeometryType` _output_get)))

(event `self.ReceiveTick`
  (params (DeltaSeconds :type "Float (single-precision)"))
  (switch `/Game/Blueprints/E_GeometryType` (`/Game/Blueprints/BP_GameInstance.CurrentGeometryType` (`self.MyGameInstance`))
    (:`NewEnumerator0`
      (if (`self.BoxIsNormalSize`)
        (if (< (`self.CurrenBoxtScale`) (`self.MaxBoxScale`))
          (bind _output_get (set `self.CurrenBoxtScale` (+ (`self.CurrenBoxtScale`) (* DeltaSeconds (`self.BoxScaleSpeed`)))))
          (`self.SetActorScale3D` (`KismetMathLibrary.Conv_DoubleToVector` _output_get)))))
    (:`NewEnumerator1`
      (`self.SetActorScale3D` (1.0 1.0 1.0) :!label _label))
    (:`NewEnumerator2`
      (goto _label))))

(event `EnhancedInput|/Game/Blueprints/Input/IA_Move`
  (params (ActionValue :type "Vector2D Structure") (ElapsedSeconds :type "Float (double-precision)") (TriggeredSeconds :type "Float (double-precision)") (InputAction :type "InputAction Object Reference" :default "/Game/Blueprints/Input/IA_Move.IA_Move"))
  (bind (_x _y) (`KismetMathLibrary.BreakVector2D` ActionValue))
  (bind (_returnvalue_roll _returnvalue_pitch _returnvalue_yaw) (`KismetMathLibrary.BreakRotator` (`self.GetControlRotation`)))
  (:`Triggered`
    (`self.AddMovementInput` (`KismetMathLibrary.GetRightVector` (`KismetMathLibrary.MakeRotator` _returnvalue_roll 0.0 _returnvalue_yaw)) _y)
    (set `self.CircleDashDirection` _y)))

(event `EnhancedInput|/Game/Blueprints/Input/IA_PauseRestart`
  (params (ActionValue :type Boolean) (ElapsedSeconds :type "Float (double-precision)") (TriggeredSeconds :type "Float (double-precision)") (InputAction :type "InputAction Object Reference" :default "/Game/Blueprints/Input/IA_PauseRestart.IA_PauseRestart"))
  (:`Completed`
    (`/Game/Blueprints/BP_GameMode.HandlePause` (`self.MyGameMode`))))

(event `EnhancedInput|/Game/Blueprints/Input/IA_SwitchPower`
  (params (ActionValue :type Boolean) (ElapsedSeconds :type "Float (double-precision)") (TriggeredSeconds :type "Float (double-precision)") (InputAction :type "InputAction Object Reference" :default "/Game/Blueprints/Input/IA_SwitchPower.IA_SwitchPower"))
  (:`Completed`
    (bind _geometrytype (`/Game/Blueprints/BP_GameMode.NextPower` (`self.MyGameMode`)))
    (`self.UpdateGeometryAttributes` _geometrytype)
    (`self.UpdateMesh` _geometrytype)))

(event `EnhancedInput|/Game/Blueprints/Input/IA_UseSkill`
  (params (ActionValue :type Boolean) (ElapsedSeconds :type "Float (double-precision)") (TriggeredSeconds :type "Float (double-precision)") (InputAction :type "InputAction Object Reference" :default "/Game/Blueprints/Input/IA_UseSkill.IA_UseSkill"))
  (:`Triggered`
    (switch `/Game/Blueprints/E_GeometryType` (`/Game/Blueprints/BP_GameInstance.CurrentGeometryType` (`self.MyGameInstance`))
      (:`NewEnumerator0`
        (`self.BoxSkill`))))
  (:`Completed`
    (switch `/Game/Blueprints/E_GeometryType` (`/Game/Blueprints/BP_GameInstance.CurrentGeometryType` (`self.MyGameInstance`))
      (:`NewEnumerator0`
        (set `self.BoxIsNormalSize` true))
      (:`NewEnumerator1`
        (`self.CircleSkill`))
      (:`NewEnumerator2`
        (`self.TriangleSkill`)))))

(fn `BoxSkill`
  (bind _returnvalue (- (`self.CurrenBoxtScale`) (* (`self.BoxScaleSpeed`) (`GameplayStatics.GetWorldDeltaSeconds`))))
  (set `self.BoxIsNormalSize` false)
  (if (> _returnvalue (`self.MinBoxScale`))
    (bind _output_get (set `self.CurrenBoxtScale` _returnvalue))
    (`self.SetActorScale3D` (`KismetMathLibrary.Conv_DoubleToVector` _output_get))))

(fn `CircleSkill`
  (`self.LaunchCharacter` (* (`self.CircleDashSpeed`) (`KismetMathLibrary.MakeVector` 0.0 (`self.CircleDashDirection`)))))

(fn `SelectMeshToRender`
  (params (HideBox :type Boolean) (HideCircle :type Boolean) (HideTriangle :type Boolean))
  (`SceneComponent.SetHiddenInGame` (`self.Cube`) HideBox false)
  (`SceneComponent.SetHiddenInGame` (`self.Sprhere`) HideCircle false)
  (`SceneComponent.SetHiddenInGame` (`self.Triangle`) HideTriangle false))

(fn `SetupController`
  (bind _asplayer_controller (cast `PlayerController` (`self.GetController`)))
  (`EnhancedInputSubsystemInterface.AddMappingContext` (pcsubsystem `EnhancedInputLocalPlayerSubsystem` _asplayer_controller) "/Game/Blueprints/Input/IMC_Player.IMC_Player" 0 (struct)))

(fn `TriangleSkill`
  (`self.Jump`))

(fn `UpdateGeometryAttributes`
  (params (GeometryType :type "/Game/Blueprints/E_GeometryType Enum" :default "NewEnumerator0"))
  (bind _charactermovement (`self.CharacterMovement`))
  (switch `/Game/Blueprints/E_GeometryType` GeometryType
    (:`NewEnumerator0`
      (set `CharacterMovementComponent.MaxWalkSpeed` (`self.Max Box Speed`) _charactermovement)
      (set `self.CurrenBoxtScale` 1.0))
    (:`NewEnumerator1`
      (set `CharacterMovementComponent.MaxWalkSpeed` (`self.Max Circle Speed`) _charactermovement))
    (:`NewEnumerator2`
      (set `CharacterMovementComponent.MaxWalkSpeed` (`self.Max Triangle Speed`) _charactermovement))))

(fn `UpdateMesh`
  (params (GeometryType :type "/Game/Blueprints/E_GeometryType Enum" :default "NewEnumerator0"))
  (switch `/Game/Blueprints/E_GeometryType` GeometryType
    (:`NewEnumerator0`
      (`self.SelectMeshToRender` false true true))
    (:`NewEnumerator1`
      (`self.SelectMeshToRender` true false true))
    (:`NewEnumerator2`
      (`self.SelectMeshToRender` true true))))

(fn `UserConstructionScript`)
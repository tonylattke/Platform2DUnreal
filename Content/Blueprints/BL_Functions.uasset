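; Blueprint function library with two general helpers for moving actors and copying vector arrays.
; UpdateActorLocation offsets a target actor by direction, speed and delta seconds, setting the location directly without sweep, so it ignores collision along the path.
; CopyVectorArray loops over an input array and returns an element-by-element copy of its locations.
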(fn `Copy Vector Array`
  (params (Array :type "Array of Vector Structure"))
  (returns (ArrayCopy :type "Array of Vector Structure"))
  (locals (LocationsCopy :type "Array of Vector Structure"))
  (for _array_element Array
    (`KismetArrayLibrary.Array_Add` (`local.LocationsCopy`) (`|Copy` _array_element)))
  (return (`local.LocationsCopy`)))

(fn `Update Actor Location`
  (params (Target :type "Actor Object Reference") (DeltaSeconds :type "Float (double-precision)") (MovementDirection :type "Vector Structure") (Speed :type "Float (double-precision)"))
  (`Actor.K2_SetActorLocation` Target (+ (`Actor.K2_GetActorLocation` Target) (* DeltaSeconds MovementDirection Speed)) false false))
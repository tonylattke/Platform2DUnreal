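; BP_Spawner is a moving spawner actor that periodically creates a random actor from a class list while near the player.
; A looping timer started on BeginPlay spawns at the spawner's location and passes each result to SaveSpawnedObject, an empty function here.
; Tick moves it along MovementDirection.
; Both spawning and movement require the player's 2D distance to be within a maximum, despite the check's visibility-based name.
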(event `self.ReceiveBeginPlay`
  (bind _asbp_game_mode (cast `/Game/Blueprints/BP_GameMode` (`GameplayStatics.GetGameMode`)))
  (set `self.MyGameMode` _asbp_game_mode)
  (`KismetSystemLibrary.K2_SetTimerDelegate` (delegate `SpawnRepeatableEvent`) (`self.TimeToSpawn`) true))

(event `SpawnRepeatableEvent`
  (`self.Spawn`))

(event `self.ReceiveTick`
  (params (DeltaSeconds :type "Float (single-precision)"))
  (if (`self.IsPlayerStillVisible`)
    (`self.UpdateLocation` DeltaSeconds)))

(fn `DistanceToPlayer`
  (returns (Result :type "Float (double-precision)"))
  (return (`KismetMathLibrary.Vector_Distance2D` (`self.K2_GetActorLocation` (`GameplayStatics.GetPlayerPawn` 0)) (`self.K2_GetActorLocation`))))

(fn `IsPlayerStillVisible`
  (returns (Result :type Boolean))
  (return (<= (`self.DistanceToPlayer`) (`self.AcceptableMaxDistance`))))

(fn `SaveSpawnedObject`
  (params (NewObject :type "Actor Object Reference")))

(fn `Spawn`
  (if (`self.IsPlayerStillVisible`)
    (bind _returnvalue (`|SpawnActorFromClass` (`KismetArrayLibrary.Array_Random` (`self.ClassToSpawn`)) (`KismetMathLibrary.MakeTransform` (`self.K2_GetActorLocation`)) "Undefined" "MultiplyWithRoot" null null))
    (`self.SaveSpawnedObject` _returnvalue)))

(fn `UpdateLocation`
  (params (DeltaTime :type "Float (double-precision)"))
  (`self.K2_SetActorLocation` (+ (`self.K2_GetActorLocation`) (* DeltaTime (`self.MovementSpeed`) (`self.MovementDirection`))) false true))

(fn `UserConstructionScript`)
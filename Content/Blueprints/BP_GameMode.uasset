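; Game mode that runs core level play: HUD setup, pause, player damage, geometry powers and level transitions.
; It relays between the level handler, which supplies powers, caps and the next level name, and the game instance, which holds current power and takes damage.
; Tick destroys the oldest registered obstacles and enemies once their arrays reach the level's caps.
; Pausing sets global time dilation to zero instead of using engine pause.
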(event `self.ReceiveBeginPlay`
  (`self.InitUI`)
  (bind _returnvalue (`GameplayStatics.GetActorOfClass` "/Game/Blueprints/BP_LevelHandler.BP_LevelHandler_C"))
  (set `self.CurrentLevelHandler` _returnvalue)
  (bind _asbp_game_instance (cast `/Game/Blueprints/BP_GameInstance` (`GameplayStatics.GetGameInstance`)))
  (set `self.MyGameInstance` _asbp_game_instance))

(event `self.ReceiveTick`
  (params (DeltaSeconds :type "Float (single-precision)"))
  (`self.ObstacleChecker`)
  (`self.EnemyChecker`))

(event `PrepareNext evelEvent`
  (bind _hud (`self.HUD`))
  (`/Game/Blueprints/BP_HUD.Show NextLevelMessage` _hud)
  (`KismetSystemLibrary.Delay` 2.0)
  (`/Game/Blueprints/BP_HUD.HideNextLevelMessage` _hud)
  (`GameplayStatics.OpenLevel` (`/Game/Blueprints/BP_LevelHandler.NextLevelName` (`self.CurrentLevelHandler`))))

(fn `AddNewPower`
  (params (PowerDescription :type "/Game/Blueprints/ST_GeometryPower Structure (by ref)"))
  (`/Game/Blueprints/BP_LevelHandler.AddPower` (`self.CurrentLevelHandler`) PowerDescription))

(fn `AddSpawnedEnemy`
  (params (NewEnemy :type "/Game/Blueprints/Enemies/BP_BaseEnemy Object Reference (by ref)"))
  (`KismetArrayLibrary.Array_Add` (`self.Enemies`) NewEnemy))

(fn `AddSpawnedObstacle`
  (params (NewObstacle :type "/Game/Blueprints/Obstacles/BP_BaseObstacle Object Reference (by ref)"))
  (`KismetArrayLibrary.Array_Add` (`self.Obstacles`) NewObstacle))

(fn `Damage Player`
  (params (Enemy :type "/Game/Blueprints/Enemies/BP_BaseEnemy Object Reference"))
  (`/Game/Blueprints/BP_GameInstance.ReceiveDamage` (`self.MyGameInstance`) (`/Game/Blueprints/Enemies/BP_BaseEnemy.DamagePoints` Enemy)))

(fn `EnemyChecker`
  (locals (ObstacleToDelete :type "/Game/Blueprints/Obstacles/BP_BaseObstacle Object Reference") (EnemyToDelete :type "/Game/Blueprints/Enemies/BP_BaseEnemy Object Reference"))
  (bind _currentlevelhandler (`self.CurrentLevelHandler`))
  (bind _enemies (`self.Enemies`))
  (`/Engine/EditorBlueprintResources/StandardMacros.IsValid` _currentlevelhandler
    (:`Is Valid`
      (if (not (`self.IsEnemyCleaning`))
        (if (>= (`KismetArrayLibrary.Array_Length` _enemies) (`/Game/Blueprints/BP_LevelHandler.MaxEnemies` _currentlevelhandler))
          (for (_array_element _array_index) _enemies
            (if (== _array_index 0)
              (set `local.EnemyToDelete` _array_element)))
          (`KismetArrayLibrary.Array_Remove` _enemies)
          (`self.K2_DestroyActor` (`local.EnemyToDelete`)))))))

(fn `HandlePause`
  (bind _output_get (set `self.IsPaused` (not (`self.IsPaused`))))
  (if _output_get
    (`GameplayStatics.SetGlobalTimeDilation` 0.0)
    (`/Game/Blueprints/BP_HUD.Show Pause` (`self.HUD`))
    (else
      (`GameplayStatics.SetGlobalTimeDilation` 1.0)
      (`/Game/Blueprints/BP_HUD.Hide Pause` (`self.HUD`)))))

(fn `InitUI`
  (bind _asbp_hud (cast `/Game/Blueprints/BP_HUD` (`PlayerController.GetHUD` (`GameplayStatics.GetPlayerController` 0))))
  (bind _output_get (set `self.HUD` _asbp_hud))
  (`/Game/Blueprints/BP_HUD.InitUI` _output_get)
  (`/Game/Blueprints/BP_HUD.ShowInGame` _output_get))

(fn `NextPower`
  (returns (GeometryType :type "/Game/Blueprints/E_GeometryType Enum"))
  (bind _currentlevelhandler (`self.CurrentLevelHandler`))
  (bind _mygameinstance (`self.MyGameInstance`))
  (bind _foundednextgeometrytype (`/Game/Blueprints/BL_Functions.CalculateNextGeometryValueAvailable` (`/Game/Blueprints/BP_LevelHandler.GeometryPowers` _currentlevelhandler) (`/Game/Blueprints/BP_GameInstance.CurrentGeometryType` _mygameinstance) 1))
  (bind _geometrydesctiption (`/Game/Blueprints/BP_LevelHandler.GetGeometryDescription` _currentlevelhandler _foundednextgeometrytype))
  (`/Game/Blueprints/BP_GameInstance.Update Power` _mygameinstance _geometrydesctiption)
  (return (`.Type_2_3770F14E43EFBDD1720B4D8BDB4D6595` (break `/Game/Blueprints/ST_GeometryPower` _geometrydesctiption))))

(fn `ObstacleChecker`
  (locals (ObstacleToDelete :type "/Game/Blueprints/Obstacles/BP_BaseObstacle Object Reference"))
  (bind _obstacles (`self.Obstacles`))
  (bind _currentlevelhandler (`self.CurrentLevelHandler`))
  (`/Engine/EditorBlueprintResources/StandardMacros.IsValid` _currentlevelhandler
    (:`Is Valid`
      (if (>= (`KismetArrayLibrary.Array_Length` _obstacles) (`/Game/Blueprints/BP_LevelHandler.MaxObstacle` _currentlevelhandler))
        (for (_array_element _array_index) _obstacles
          (if (== _array_index 0)
            (set `local.ObstacleToDelete` _array_element)
            (break)))
        (`KismetArrayLibrary.Array_Remove` (`self.Obstacles`))
        (`self.K2_DestroyActor` (`local.ObstacleToDelete`))))))

(fn `UserConstructionScript`)
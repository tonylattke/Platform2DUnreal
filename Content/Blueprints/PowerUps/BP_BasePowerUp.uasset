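; Base power-up pickup actor that grants the player a new power when touched.
; It caches BP_GameMode on BeginPlay and reacts when BP_Player overlaps its Collision component.
; The overlap passes PowerDescription to the game mode's AddNewPower and briefly shows the HUD's unlock notice.
; The actor destroys itself only after that delayed notice hides, with no guard against repeat overlaps meanwhile.
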(event `self.ReceiveBeginPlay`
  (bind _asbp_game_mode (cast `/Game/Blueprints/BP_GameMode` (`GameplayStatics.GetGameMode`)))
  (set `self.MyGame Mode` _asbp_game_mode))

(event `self.Collision.OnComponentBeginOverlap`
  (params (OverlappedComponent :type "PrimitiveComponent Object Reference") (OtherActor :type "Actor Object Reference") (OtherComp :type "PrimitiveComponent Object Reference") (OtherBodyIndex :type Integer) (bFromSweep :type Boolean) (SweepResult :type "HitResult Structure (by ref)"))
  (bind _mygame_mode (`self.MyGame Mode`))
  (bind _hud (`/Game/Blueprints/BP_GameMode.HUD` _mygame_mode))
  (cast `/Game/Blueprints/BP_Player` OtherActor)
  (`/Game/Blueprints/BP_GameMode.AddNewPower` _mygame_mode (`self.Power Description`))
  (`/Game/Blueprints/BP_HUD.Show NewPowerUnlocked` _hud)
  (`KismetSystemLibrary.Delay` 2.0)
  (`/Game/Blueprints/BP_HUD.HideNewPowerUnlocked` _hud)
  (`self.K2_DestroyActor`))

(fn `UserConstructionScript`)
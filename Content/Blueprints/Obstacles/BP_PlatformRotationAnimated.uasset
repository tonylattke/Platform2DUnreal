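; Rotating platform obstacle that swings its child actor back and forth, reversing direction at a fixed interval.
; Each Tick adds RotationDirection scaled by RotationSpeed and delta time to the world rotation of the BPMesh child actor.
; A looping timer started on BeginPlay negates RotationDirection every TimeInterval.
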(event `self.ReceiveBeginPlay`
  (`parent.ReceiveBeginPlay`)
  (`KismetSystemLibrary.K2_SetTimerDelegate` (delegate `MovementDirectionChanger`) (`self.TimeInterval`) true))

(event `MovementDirectionChanger`
  (`self.NegateDirection`))

(event `self.ReceiveTick`
  (params (DeltaSeconds :type "Float (single-precision)"))
  (bind _childactor (`ChildActorComponent.ChildActor` (`self.BP_Mesh`)))
  (`parent.ReceiveTick` DeltaSeconds)
  (`self.K2_SetActorRotation` _childactor (`KismetMathLibrary.MakeRotator` (+ (.roll (`self.K2_GetActorRotation` _childactor)) (.roll (* (* (`self.RotationDirection`) (`self.RotationSpeed`)) DeltaSeconds))) (+ (.pitch (`self.K2_GetActorRotation` _childactor)) (.pitch (* (* (`self.RotationDirection`) (`self.RotationSpeed`)) DeltaSeconds))) (+ (.yaw (`self.K2_GetActorRotation` _childactor)) (.yaw (* (* (`self.RotationDirection`) (`self.RotationSpeed`)) DeltaSeconds)))) false))

(fn `NegateDirection`
  (set `self.RotationDirection` (* (`self.RotationDirection`) -1.0)))

(fn `UserConstructionScript`
  (`parent.UserConstructionScript`))
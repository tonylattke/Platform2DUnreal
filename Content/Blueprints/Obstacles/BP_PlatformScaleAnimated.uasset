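; BP_PlatformScaleAnimated is an obstacle platform that continuously grows and shrinks over time.
; Each Tick adds ScaleSpeed times ScaleDirection, scaled by delta time, to the scale of the actor spawned by its BPMesh child actor component.
; A looping timer set on BeginPlay negates ScaleDirection every TimeInterval seconds, producing the back-and-forth scaling.
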(event `self.ReceiveBeginPlay`
  (`parent.ReceiveBeginPlay`)
  (`KismetSystemLibrary.K2_SetTimerDelegate` (delegate `MovementDirectionChanger`) (`self.TimeInterval`) true))

(event `MovementDirectionChanger`
  (`self.NegateDirection`))

(event `self.ReceiveTick`
  (params (DeltaSeconds :type "Float (single-precision)"))
  (bind _childactor (`ChildActorComponent.ChildActor` (`self.BP_Mesh`)))
  (`parent.ReceiveTick` DeltaSeconds)
  (`self.SetActorScale3D` _childactor (+ (`self.GetActorScale3D` _childactor) (* DeltaSeconds (`self.ScaleSpeed`) (`self.ScaleDirection`)))))

(fn `NegateDirection`
  (set `self.ScaleDirection` (* (`self.ScaleDirection`) -1.0)))

(fn `UserConstructionScript`
  (`parent.UserConstructionScript`))